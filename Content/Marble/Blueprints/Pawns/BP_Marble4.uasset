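; Player-controlled marble pawn that rolls by physics force and overheats as it is pushed.
; Enhanced Input applies forces along the camera's forward and right vectors and drives spring-arm yaw and zoom.
; Movement input accumulates signed Heat, blocking further force once its magnitude reaches MaxHeat, while Tick cools it when movement input is zero.
; A dynamic granite material's albedo tint shifts from white toward magenta with heat.
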(event Input|EnhancedActionEvents|EnhancedInputActionIA_CameraLeftRight
  (params (ActionValue :type Float%20%28double-precision%29) (ElapsedSeconds :type Float%20%28double-precision%29) (TriggeredSeconds :type Float%20%28double-precision%29) (InputAction :type Input%20Action%20Object%20Reference :default "/Game/Marble/Inputs/Marble4/IA_CameraLeftRight.IA_CameraLeftRight"))
  (bind _springarm (Variables|Default|GetSpringArm))
  (bind _relativerotation (Variables|/Script/Engine.SceneComponent|GetRelativeRotation _springarm))
  (Transformation|SetRelativeRotation (Variables|Default|GetSpringArm) (Math|Rotator|MakeRotator 0.0 (.pitch _relativerotation) (+ (.yaw _relativerotation) (* ActionValue (Variables|Default|GetCamera%20Rotation)))) false false))

(event Input|EnhancedActionEvents|EnhancedInputActionIA_LeftRight
  (params (ActionValue :type Float%20%28double-precision%29) (ElapsedSeconds :type Float%20%28double-precision%29) (TriggeredSeconds :type Float%20%28double-precision%29) (InputAction :type Input%20Action%20Object%20Reference :default "/Game/Marble/Inputs/Marble4/IA_LeftRight.IA_LeftRight"))
  (:Triggered
    (Variables|Default|SetAction%20Value ActionValue)
    (if (CallFunction|MarbleNotTooHot?)
      (Physics|AddForce (Variables|Default|GetMarble) (* (* (Variables|Default|GetAction%20Value) (Variables|Default|GetForce)) (Math|Vector|GetRightVector (Variables|Default|GetCamera))) "None" false)
      (Variables|Default|SetHeat (+ (Variables|Default|GetHeat) (Variables|Default|GetAction%20Value)))
      (CallFunction|UpdateHeatColor)))
  (:Completed
    (Variables|Default|SetAction%20Value 0.0)))

(event Input|EnhancedActionEvents|EnhancedInputActionIA_Forward
  (params (ActionValue :type Float%20%28double-precision%29) (ElapsedSeconds :type Float%20%28double-precision%29) (TriggeredSeconds :type Float%20%28double-precision%29) (InputAction :type Input%20Action%20Object%20Reference :default "/Game/Marble/Inputs/Marble4/IA_Forward.IA_Forward"))
  (:Triggered
    (Variables|Default|SetAction%20Value ActionValue)
    (if (CallFunction|MarbleNotTooHot?)
      (Physics|AddForce (Variables|Default|GetMarble) (* (* (Variables|Default|GetAction%20Value) (Variables|Default|GetForce)) (Math|Vector|GetForwardVector (Variables|Default|GetCamera))) "None" false)
      (Variables|Default|SetHeat (+ (Variables|Default|GetHeat) (Variables|Default|GetAction%20Value)))
      (CallFunction|UpdateHeatColor)))
  (:Completed
    (Variables|Default|SetAction%20Value 0.0)))

(event Input|EnhancedActionEvents|EnhancedInputActionIA_CameraZoomInOut
  (params (ActionValue :type Float%20%28double-precision%29) (ElapsedSeconds :type Float%20%28double-precision%29) (TriggeredSeconds :type Float%20%28double-precision%29) (InputAction :type Input%20Action%20Object%20Reference :default "/Game/Marble/Inputs/Marble4/IA_CameraZoomInOut.IA_CameraZoomInOut"))
  (bind _output_get (Variables|Default|SetSpring%20Arm%20Length (+ (* ActionValue (Variables|Default|GetZoom%20Factor)) (Variables|Default|GetSpring%20Arm%20Length))))
  (Variables|/Script/Engine.SpringArmComponent|SetTargetArmLength (Variables|Default|GetSpringArm) _output_get))

(event EventTick
  (params (DeltaSeconds :type Float%20%28single-precision%29))
  (if (== (Variables|Default|GetAction%20Value) 0.0)
    (CallFunction|CoolMarble)
    (CallFunction|UpdateHeatColor)))

(event EventBeginPlay
  (bind _asplayer_controller (Utilities|Casting|CastToPlayerController (Pawn|GetController)))
  (Utilities|IsValid _asplayer_controller
    (:Is%20Valid
      (Input|AddMappingContext (PlayerController|LocalPlayerSubsystems|GetEnhancedInputLocalPlayerSubsystem _asplayer_controller) "/Game/Marble/Inputs/Marble4/IMC_Marble.IMC_Marble" 0 "(bIgnoreAllPressedKeysUntilRelease=True,bForceImmediately=False,bNotifyUserSettings=False)")
      (bind _returnvalue (Rendering|Material|CreateDynamicMaterialInstance (Variables|Default|GetMarble) 0 "/Game/Megascans/Surfaces/Belvedere_Granite_wkvjefyl/MI_Belvedere_Granite_wkvjefyl_2K.MI_Belvedere_Granite_wkvjefyl_2K" "None" :!class /Script/Engine.PrimitiveComponent))
      (bind _output_get (Variables|Default|SetMarble%20Material _returnvalue))
      (Rendering|Material|SetMaterial (Variables|Default|GetMarble) 0 _output_get))))

(fn ConstructionScript)

(fn Accelerate
  (params (A :type Float%20%28double-precision%29))
  (Physics|AddForce (Variables|Default|GetMarble) (* (* A (Variables|Default|GetForce)) (Math|Vector|GetForwardVector (Variables|Default|GetCamera))) "None" false))

(fn MarbleNotTooHot?
  (return (< (Math|Float|Absolute(Float) (Variables|Default|GetHeat)) (Variables|Default|GetMax%20Heat))))

(fn CoolMarble
  (if (< (Variables|Default|GetHeat) 0.0)
    (Variables|Default|SetHeat (+ (Variables|Default|GetHeat) (Variables|Default|GetHeat%20Cooling)))
    (else
      (Variables|Default|SetHeat (- (Variables|Default|GetHeat) (Variables|Default|GetHeat%20Cooling))))))

(fn UpdateHeatColor
  (Rendering|Material|SetVectorParameterValueonMaterials (Variables|Default|GetMarble) "Albedo Tint" (Math|Vector|MakeVector 1.0 (- 1.0 (Math|Float|Absolute(Float) (/ (Variables|Default|GetHeat) (Variables|Default|GetMax%20Heat)))) 1.0)))