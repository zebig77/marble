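; BP_DebugMarble is a debug marble pawn that the player rolls around with physics forces.
; Enhanced Input forward and left/right actions push the Marble along the camera's axes, scaled by Force.
; Each tick, once the marble has moved beyond a small tolerance, the spring arm yaws toward the travel direction, keeping its pitch.
; MarbleNotTooHot is a stub that always returns false.
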(event Input|EnhancedActionEvents|EnhancedInputActionIA_LeftRight
  (params (ActionValue :type Float%20%28double-precision%29) (ElapsedSeconds :type Float%20%28double-precision%29) (TriggeredSeconds :type Float%20%28double-precision%29) (InputAction :type Input%20Action%20Object%20Reference :default "/Game/Marble/Inputs/Marble4/IA_LeftRight.IA_LeftRight"))
  (Physics|AddForce (Variables|Default|GetMarble) (* (* ActionValue (Variables|Default|GetForce)) (Math|Vector|GetRightVector (Variables|Default|GetCamera))) "None" false))

(event Input|EnhancedActionEvents|EnhancedInputActionIA_Forward
  (params (ActionValue :type Float%20%28double-precision%29) (ElapsedSeconds :type Float%20%28double-precision%29) (TriggeredSeconds :type Float%20%28double-precision%29) (InputAction :type Input%20Action%20Object%20Reference :default "/Game/Marble/Inputs/Marble4/IA_Forward.IA_Forward"))
  (Physics|AddForce (Variables|Default|GetMarble) (* (* ActionValue (Variables|Default|GetForce)) (Math|Vector|GetForwardVector (Variables|Default|GetCamera))) "None" false))

(event EventTick
  (params (DeltaSeconds :type Float%20%28single-precision%29))
  (if (Utilities|Operators|NotEqual(!=) (Variables|Default|GetMarble%20Previous%20location) (Transformation|GetWorldLocation (Variables|Default|GetMarble)) 0.5)
    (Transformation|SetRelativeRotation (Variables|Default|GetSpringArm) (Math|Rotator|MakeRotator 0.0 (.pitch (Variables|/Script/Engine.SceneComponent|GetRelativeRotation (Variables|Default|GetSpringArm))) (.yaw (Math|Rotator|FindLookatRotation (Variables|Default|GetMarble%20Previous%20location) (Transformation|GetWorldLocation (Variables|Default|GetMarble))))) false false)
    (Variables|Default|SetMarble%20Previous%20location (Transformation|GetWorldLocation (Variables|Default|GetMarble)))))

(event EventBeginPlay
  (bind _asplayer_controller (Utilities|Casting|CastToPlayerController (Pawn|GetController)))
  (Utilities|IsValid _asplayer_controller
    (:Is%20Valid
      (Input|AddMappingContext (PlayerController|LocalPlayerSubsystems|GetEnhancedInputLocalPlayerSubsystem _asplayer_controller) "/Game/Marble/Inputs/Marble4/IMC_Marble.IMC_Marble" 0 "(bIgnoreAllPressedKeysUntilRelease=True,bForceImmediately=False,bNotifyUserSettings=False)")
      (Variables|Default|SetMarble%20Previous%20location (Transformation|GetWorldLocation (Variables|Default|GetMarble))))))

(fn ConstructionScript)

(fn MarbleNotTooHot?
  (return false))