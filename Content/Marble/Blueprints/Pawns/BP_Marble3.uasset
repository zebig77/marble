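; BP_Marble3 is a player pawn that rolls a physics marble with a trailing spring-arm camera.
; BeginPlay adds the IMC_Marble Enhanced Input context, and the forward and left/right actions apply scaled forces along the scene root's axes, independent of the camera.
; Each tick derives a heading from marble velocity and arrow relative location, snaps the arrow to it, and eases spring-arm yaw and downward-offset pitch toward it with FInterpTo.
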(event Input|EnhancedActionEvents|EnhancedInputActionIA_LeftRight
  (params (ActionValue :type Float%20%28double-precision%29) (ElapsedSeconds :type Float%20%28double-precision%29) (TriggeredSeconds :type Float%20%28double-precision%29) (InputAction :type Input%20Action%20Object%20Reference :default "/Game/Marble/Inputs/IA_LeftRight.IA_LeftRight"))
  (Physics|AddForce (Variables|Default|GetMarble) (* (* ActionValue (Variables|Default|GetForce)) (Math|Vector|GetRightVector (Variables|Default|GetDefaultSceneRoot))) "None" false))

(event Input|EnhancedActionEvents|EnhancedInputActionIA_Forward
  (params (ActionValue :type Float%20%28double-precision%29) (ElapsedSeconds :type Float%20%28double-precision%29) (TriggeredSeconds :type Float%20%28double-precision%29) (InputAction :type Input%20Action%20Object%20Reference :default "/Game/Marble/Inputs/IA_Forward.IA_Forward"))
  (Physics|AddForce (Variables|Default|GetMarble) (* (* ActionValue (Variables|Default|GetForce)) (Math|Vector|GetForwardVector (Variables|Default|GetDefaultSceneRoot))) "None" false))

(event EventTick
  (params (DeltaSeconds :type Float%20%28single-precision%29))
  (bind _returnvalue (Utilities|Time|GetWorldDeltaSeconds))
  (bind _springarm (Variables|Default|GetSpringArm))
  (bind _returnvalue_2 (Transformation|GetWorldRotation _springarm))
  (bind _output_get (Variables|Default|SetForward%20Direction (Math|Vector|GetUnitDirection(Vector) (Variables|/Script/Engine.SceneComponent|GetRelativeLocation (Variables|Default|GetArrow)) (Transformation|GetComponentVelocity (Variables|Default|GetMarble)))))
  (Transformation|SetWorldRotation (Variables|Default|GetArrow) (Math|Rotator|MakeRotationfromAxes _output_get "0, 0, 0" "0, 0, 0") false false)
  (Transformation|SetWorldRotation (Variables|Default|GetSpringArm) (Math|Rotator|MakeRotator 0.0 (Math|Interpolation|FInterpTo (.pitch _returnvalue_2) (- (.Pitch (Math|Rotator|BreakRotator (Math|Rotator|MakeRotationfromAxes _output_get "0, 0, 0" "0, 0, 0"))) 15.0) _returnvalue 2.0) (Math|Interpolation|FInterpTo (.yaw _returnvalue_2) (.Yaw (Math|Rotator|BreakRotator (Math|Rotator|MakeRotationfromAxes _output_get "0, 0, 0" "0, 0, 0"))) _returnvalue 2.0)) false false))

(event EventBeginPlay
  (bind _asplayer_controller (Utilities|Casting|CastToPlayerController (Pawn|GetController)))
  (Utilities|IsValid _asplayer_controller
    (:Is%20Valid
      (Input|AddMappingContext (PlayerController|LocalPlayerSubsystems|GetEnhancedInputLocalPlayerSubsystem _asplayer_controller) "/Game/Marble/Inputs/IMC_Marble.IMC_Marble" 0 "(bIgnoreAllPressedKeysUntilRelease=True,bForceImmediately=False,bNotifyUserSettings=False)"))))

(fn ConstructionScript)