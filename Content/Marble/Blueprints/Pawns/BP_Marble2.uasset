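; BP_Marble2 is a player-controlled marble pawn, moved by physics forces.
; BeginPlay registers the IMC_Marble Enhanced Input context, and forward and left/right actions push the Marble along DefaultSceneRoot's axes, scaled by Force.
; Each tick, Arrow sweeps to the marble and orients along its travel direction, derived from the previous location, using axes built with trigonometry and a cross product.
; An unconnected SpringArm rotation node is never run.
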(event Input|EnhancedActionEvents|EnhancedInputActionIA_LeftRight
  (params (ActionValue :type Float%20%28double-precision%29) (ElapsedSeconds :type Float%20%28double-precision%29) (TriggeredSeconds :type Float%20%28double-precision%29) (InputAction :type Input%20Action%20Object%20Reference :default "/Game/Marble/Inputs/IA_LeftRight.IA_LeftRight"))
  (Physics|AddForce (Variables|Default|GetMarble) (* (* ActionValue (Variables|Default|GetForce)) (Math|Vector|GetRightVector (Variables|Default|GetDefaultSceneRoot))) "None" false))

(event Input|EnhancedActionEvents|EnhancedInputActionIA_Forward
  (params (ActionValue :type Float%20%28double-precision%29) (ElapsedSeconds :type Float%20%28double-precision%29) (TriggeredSeconds :type Float%20%28double-precision%29) (InputAction :type Input%20Action%20Object%20Reference :default "/Game/Marble/Inputs/IA_Forward.IA_Forward"))
  (Physics|AddForce (Variables|Default|GetMarble) (* (* ActionValue (Variables|Default|GetForce)) (Math|Vector|GetForwardVector (Variables|Default|GetDefaultSceneRoot))) "None" false))

(event EventTick
  (params (DeltaSeconds :type Float%20%28single-precision%29))
  (Transformation|SetWorldLocation (Variables|Default|GetArrow) (Transformation|GetWorldLocation (Variables|Default|GetMarble)) true false)
  (Transformation|SetWorldRotation (Variables|Default|GetArrow) (Math|Rotator|MakeRotationfromAxes (Math|Vector|GetUnitDirection(Vector) (Variables|Default|GetPrevious%20Location) (Transformation|GetWorldLocation (Variables|Default|GetMarble))) (Math|Vector|MakeVector (Class|KismetMathLibrary|DegAcos (+ (Class|KismetMathLibrary|DegAtan2 (.Y (Math|Vector|BreakVector (Math|Vector|GetUnitDirection(Vector) (Variables|Default|GetPrevious%20Location) (Transformation|GetWorldLocation (Variables|Default|GetMarble))))) (.X (Math|Vector|BreakVector (Math|Vector|GetUnitDirection(Vector) (Variables|Default|GetPrevious%20Location) (Transformation|GetWorldLocation (Variables|Default|GetMarble)))))) 9e+01)) (Math|Trig|Sin(Degrees) (+ (Class|KismetMathLibrary|DegAtan2 (.Y (Math|Vector|BreakVector (Math|Vector|GetUnitDirection(Vector) (Variables|Default|GetPrevious%20Location) (Transformation|GetWorldLocation (Variables|Default|GetMarble))))) (.X (Math|Vector|BreakVector (Math|Vector|GetUnitDirection(Vector) (Variables|Default|GetPrevious%20Location) (Transformation|GetWorldLocation (Variables|Default|GetMarble)))))) 9e+01)) 0.0) (Math|Vector|CrossProduct (Math|Vector|GetUnitDirection(Vector) (Variables|Default|GetPrevious%20Location) (Transformation|GetWorldLocation (Variables|Default|GetMarble))) (Math|Vector|MakeVector (Class|KismetMathLibrary|DegAcos (+ (Class|KismetMathLibrary|DegAtan2 (.Y (Math|Vector|BreakVector (Math|Vector|GetUnitDirection(Vector) (Variables|Default|GetPrevious%20Location) (Transformation|GetWorldLocation (Variables|Default|GetMarble))))) (.X (Math|Vector|BreakVector (Math|Vector|GetUnitDirection(Vector) (Variables|Default|GetPrevious%20Location) (Transformation|GetWorldLocation (Variables|Default|GetMarble)))))) 9e+01)) (Math|Trig|Sin(Degrees) (+ (Class|KismetMathLibrary|DegAtan2 (.Y (Math|Vector|BreakVector (Math|Vector|GetUnitDirection(Vector) (Variables|Default|GetPrevious%20Location) (Transformation|GetWorldLocation (Variables|Default|GetMarble))))) (.X (Math|Vector|BreakVector (Math|Vector|GetUnitDirection(Vector) (Variables|Default|GetPrevious%20Location) (Transformation|GetWorldLocation (Variables|Default|GetMarble)))))) 9e+01)) 0.0))) false false)
  (Variables|Default|SetPrevious%20Location (Transformation|GetWorldLocation (Variables|Default|GetMarble))))

(event EventBeginPlay
  (bind _asplayer_controller (Utilities|Casting|CastToPlayerController (Pawn|GetController)))
  (Utilities|IsValid _asplayer_controller
    (:Is%20Valid
      (Input|AddMappingContext (PlayerController|LocalPlayerSubsystems|GetEnhancedInputLocalPlayerSubsystem _asplayer_controller) "/Game/Marble/Inputs/IMC_Marble.IMC_Marble" 0 "(bIgnoreAllPressedKeysUntilRelease=True,bForceImmediately=False,bNotifyUserSettings=False)")
      (Variables|Default|SetPrevious%20Location (Transformation|GetWorldLocation (Variables|Default|GetMarble))))))

(fn ConstructionScript)